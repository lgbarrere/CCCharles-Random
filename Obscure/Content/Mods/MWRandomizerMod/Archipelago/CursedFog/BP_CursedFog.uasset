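; BP_CursedFog is a cursed fog volume for the Archipelago randomizer mod that clears when Fogbane is received.
; Each tick it derives FogDensity and a near-fog flag from the camera's distance to the sphere's bounds, scaled by FogFade.
; FogbaneReceived runs a timeline that lowers the fade on the density and dynamic sphere material, stops and detaches the particles, then destroys the actor.
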(event Custom|FogbaneReceived
  (bind _fadevalue (Timeline|Timeline_0 PlayFromStart)
    (:Update
      (CallFunction|ClearFog _fadevalue))
    (:Finished
      (Actor|DestroyActor))))

(event EventBeginPlay
  (bind _returnvalue (Rendering|Material|CreateDynamicMaterialInstance "/Game/Mods/MWRandomizerMod/Archipelago/CursedFog/M_CursedFog.M_CursedFog" "None" "None" :!class /Script/Engine.KismetMaterialLibrary))
  (Variables|Default|SetCursedFogMID _returnvalue)
  (Rendering|Material|SetMaterial (Variables|Default|GetCurseFogSphere) 0 (Variables|Default|GetCursedFogMID)))

(event EventTick
  (params (DeltaSeconds :type Float%20%28single-precision%29))
  (CallFunction|CheckNearPlayer))

(fn ConstructionScript)

(fn PrinttoModLoader
  (params (Message :type String)))

(fn CheckNearPlayer
  (bind _cursefogsphere (Variables|Default|GetCurseFogSphere))
  (bind (_origin _boxextent _sphereradius) (Collision|GetComponentBounds _cursefogsphere))
  (bind _output_get (Variables|Default|SetFogDensity (* (Math|Float|Clamp(Float) (- 1.0 (/ (- (Math|Vector|Distance(Vector) (CallFunction|GetWorldPlayerViewLocation) _origin) _sphereradius) (Variables|Default|GetInteractionDistance)))) (Variables|Default|GetFogFade))))
  ;[1 1 1] Invert IsPlayerNearFog when it does not match the previous condition
  (if (Math|Boolean|NotEqual(Boolean) (> _output_get 0.0) (Variables|Default|GetIsPlayerNearFog))
    (Variables|Default|SetIsPlayerNearFog (not (Variables|Default|GetIsPlayerNearFog)))
    (return)))

(fn GetWorldPlayerViewLocation
  (bind _returnvalue (Viewport|GetViewportSize))
  (bind _returnvalue_2 (/ _returnvalue 2.0))
  (bind (_x _y) (Math|Vector2D|BreakVector2D _returnvalue_2))
  (return (.WorldLocation (Class|PlayerController|DeprojectScreenPositiontoWorld (Game|GetPlayerController 0) _x _y))))

(fn ClearFog
  (params (Fade :type Float%20%28single-precision%29))
  (Variables|Default|SetFogFade Fade)
  ;[1 1 1] Stop particles spawn (let them disappear)
  (Niagara|SetNiagaraVariable(Float) (Variables|Default|GetCursedFogParticles) "User.SpawnRate" 0.0)
  (Transformation|DetachFromComponent (Variables|Default|GetCursedFogParticles) "KeepWorld" "KeepWorld" "KeepWorld" true)
  (Rendering|Material|SetScalarParameterValue (Variables|Default|GetCursedFogMID) "GlobalFade" (/ (Variables|Default|GetFogFade) 2.0) :!class /Script/Engine.MaterialInstanceDynamic)
  (Rendering|Material|SetMaterial (Variables|Default|GetCurseFogSphere) 0 (Variables|Default|GetCursedFogMID))
  (return))