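; Death Duck actor for the MWRandomizer mod that destroys colliding actors whose class is in its randomized list.
; Physics-simulated collisions raise Hit events, which match the other actor's class display name against RandomizedClasses, print to the mod loader and destroy it.
; BeginPlay enables player input.
; Unconnected nodes sketch an Archipelago hint or sent-item collect message and disabling body and head physics, but never run.
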(event Custom|PrintToModLoader
  (params (Message :type String)))

(event EventBeginPlay
  (Input|EnableInput (Game|GetPlayerController 0)))

(event Collision|EventHit
  (params (MyComp :type Primitive%20Component%20Object%20Reference) (Other :type Actor%20Object%20Reference) (OtherComp :type Primitive%20Component%20Object%20Reference) (bSelfMoved :type Boolean) (HitLocation :type Vector :default "0, 0, 0") (HitNormal :type Vector :default "0, 0, 0") (NormalImpulse :type Vector :default "0, 0, 0") (Hit :type Hit%20Result%20Structure%20%28by%20ref%29))
  ;[1 1 1] The physics simulations are enabled for DeathDuck's collisions, that triggers a Event Hit while colliding
  (for _array_element (Variables|Default|GetRandomizedClasses)
    (if (Utilities|Enum|Equal(Enum) _array_element (Utilities|GetClassDisplayName (Utilities|GetClass Other)))
      (CallFunction|PrinttoModLoader "unexpected ?")
      (Actor|DestroyActor Other))))

(fn ConstructionScript)