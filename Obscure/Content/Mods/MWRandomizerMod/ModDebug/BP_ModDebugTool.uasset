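; Debug tool actor for the MWRandomizer mod, offering developer cheats and inspection through overlay buttons and hotkeys that share the same logic.
; BeginPlay creates both widgets, binds buttons and adds a floating pawn movement component for speed boost.
; A screen-center line trace logs actor and collision details and alternately fills two slots for location swapping.
; Other tools teleport the player, list and visit pickups, edit inventory, mark locations and adjust a test fog.
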(event Custom|RemoveFromInventoryEvent
  ;[1 1 1] Key mapping section
  ;;[0 0 0] Press "-" to remove an item from the inventory
  (CallFunction|AllItemstoInventory -1))

(event Custom|PrintToModLoader
  (params (Message :type String)))

(event Custom|ShowVisualFeeback
  ;[1 1 1] Match the clicked buttons with expected events
  (CallFunction|ShowVisualFeedbackEvent))

(event Custom|ToLockpicksMissionEvent
  ;[1 1 1] Key mapping section
  ;;[0 0 0] Press "L" to be teleported to the Lockpicks mission
  (Transformation|SetActorLocation (Game|Player|GetPlayerPawn 0) (Variables|Default|GetLockpicksMissionLocation) false false))

(event Custom|SkipTutorial
  ;[1 1 1] Match the clicked buttons with expected events
  (CallFunction|SkipTutorialEvent))

(event Custom|BackToTrainEvent
  ;[1 1 1] Key mapping section
  ;;[0 0 0] Press "B" to be teleported back to the Train
  (Transformation|SetActorLocation (Game|Player|GetPlayerPawn 0) "0, 0, 0" false false))

(event Custom|ToLockpicksMission
  ;[1 1 1] Match the clicked buttons with expected events
  (CallFunction|ToLockpicksMissionEvent))

(event Custom|Swap2ActorsEvent
  (bind _itemactor2 (Variables|Default|GetItemActor2))
  (bind _itemactor1 (Variables|Default|GetItemActor1))
  ;[1 1 1] Key mapping section
  ;;[0 0 0] Press "1" to swap 2 selected Actors with "R"
  ;;;[1 1 1] Check the actors to swap are valid
  (if (and (Utilities|IsValid (Variables|Default|GetItemActor1)) (Utilities|IsValid (Variables|Default|GetItemActor2)))
    (Variables|Default|SetTmpActor1Location (Transformation|GetActorLocation _itemactor1)) ; Store the location of the Actor1\nto not loose it
    (Transformation|SetActorLocation _itemactor1 (Transformation|GetActorLocation _itemactor2) false false)
    (Transformation|SetActorLocation _itemactor2 (Variables|Default|GetTmpActor1Location) false false)))

(event Custom|BackToTrain
  ;[1 1 1] Match the clicked buttons with expected events
  (CallFunction|BacktoTrainEvent))

(event Custom|ListAllPickableItemsEvent
  ;[1 1 1] Key mapping section
  ;;[0 0 0] Press "2" to virtually list all pickable items (laggy) and to teleport on each with "3"
  (bind _outactors (Actor|GetAllActorsOfClass "/Game/_GAME/Blueprints/ItemPickup.ItemPickup_C"))
  (bind _output_get (Variables|Default|SetAllPickupItems _outactors))
  (for _array_element _output_get
    ;;[0.4243 0.7148 1] Print each found item information in the mod loader
    (CallFunction|PrinttoModLoader (Utilities|GetDisplayName _array_element))
    (CallFunction|PrinttoModLoader (Utilities|GetClassDisplayName (Utilities|GetClass _array_element)))
    (CallFunction|PrinttoModLoader (Utilities|String|ToString(Vector) (Transformation|GetActorLocation _array_element))))
  (Variables|Default|SetItemIndex 0))

(event Custom|Swap2Actors
  ;[1 1 1] Match the clicked buttons with expected events
  (CallFunction|Swap2ActorsEvent))

(event Custom|ToNextListedItemEvent
  ;[1 1 1] Key mapping section
  ;;[0 0 0] Press "3" to teleport to the next listed item with "2"
  (CallFunction|TeleportPlayertoNextItem))

(event Custom|ListPickableItems
  ;[1 1 1] Match the clicked buttons with expected events
  (CallFunction|ListAllPickableItemsEvent))

(event Custom|AddToInventoryEvent
  ;[1 1 1] Key mapping section
  ;;[0 0 0] Press "+" to add an item to the inventory
  (CallFunction|AllItemstoInventory 8))

(event Custom|ToNextListedItem
  ;[1 1 1] Match the clicked buttons with expected events
  (CallFunction|ToNextListedItemEvent))

(event Custom|AddToInventory
  ;[1 1 1] Match the clicked buttons with expected events
  (CallFunction|AddtoInventoryEvent))

(event Custom|RemoveFromInventory
  ;[1 1 1] Match the clicked buttons with expected events
  (CallFunction|RemovefromInventoryEvent))

(event Custom|SelectItem
  ;[1 1 1] Match the clicked buttons with expected events
  (CallFunction|SelectItemEvent))

(event Custom|SpeedBoostClicked
  ;[1 1 1] Match the clicked buttons with expected events
  (CallFunction|SpeedBoostEvent))

(event Custom|SelectItemEvent
  ;[1 1 1] Key mapping section
  ;;[0 0 0] Press "R" to select an item and to get its references
  (if true
    (CallFunction|SetClickedActor)))

(event Custom|ShowVisualFeedbackEvent
  (bind _moddebugui (Variables|Default|GetModDebugUI))
  ;[1 1 1] Key mapping section
  ;;[0 0 0] Press "V" to show the Visual Feedback
  (bind _output_get (Variables|Default|SetEnableVisualFeedback (not (Variables|Default|GetEnableVisualFeedback))))
  (if _output_get
    (Widget|SetVisibility _moddebugui "SelfHitTestInvisible")
    (else
      (Widget|SetVisibility _moddebugui "Hidden"))))

(event Custom|SpeedBoostEvent
  (bind _pawnmovementcomponent (Variables|Default|GetPawnMovementComponent))
  ;[1 1 1] Key mapping section
  ;;[0 0 0] Press "F" to enable/disable the speed boost
  (bind _output_get (Variables|Default|SetEnableSpeedBoost (not (Variables|Default|GetEnableSpeedBoost))))
  (if _output_get
    (Variables|/Script/Engine.FloatingPawnMovement|SetMaxSpeed _pawnmovementcomponent 2e+05)
    (Variables|/Script/Engine.FloatingPawnMovement|SetAcceleration _pawnmovementcomponent 4e+03)
    (Variables|/Script/Engine.FloatingPawnMovement|SetDeceleration _pawnmovementcomponent 8e+03)
    (else
      (Variables|/Script/Engine.FloatingPawnMovement|SetMaxSpeed _pawnmovementcomponent 8e+02)
      (Variables|/Script/Engine.FloatingPawnMovement|SetAcceleration _pawnmovementcomponent 1e+06)
      (Variables|/Script/Engine.FloatingPawnMovement|SetDeceleration _pawnmovementcomponent 8e+03))))

(event Custom|SetButtonEvents
  ;[1 1 1] Match the clicked buttons with expected events
  (EventDispatchers|BindEventtoSpeedBoostClicked (Variables|Default|GetOverlay) (delegate Custom|SpeedBoostClicked))
  (EventDispatchers|BindEventtoSelectItemClicked (Variables|Default|GetOverlay) (delegate Custom|SelectItem))
  (EventDispatchers|BindEventtoShowVisualFeedbackClicked (Variables|Default|GetOverlay) (delegate Custom|ShowVisualFeeback))
  (EventDispatchers|BindEventtoSkipTutorialClicked (Variables|Default|GetOverlay) (delegate Custom|SkipTutorial))
  (EventDispatchers|BindEventtoToLockpickMissionClicked (Variables|Default|GetOverlay) (delegate Custom|ToLockpicksMission))
  (EventDispatchers|BindEventtoBacktoTrainClicked (Variables|Default|GetOverlay) (delegate Custom|BackToTrain))
  (EventDispatchers|BindEventtoSwap2ActorsClicked (Variables|Default|GetOverlay) (delegate Custom|Swap2Actors))
  (EventDispatchers|BindEventtoListPickableItemsClicked (Variables|Default|GetOverlay) (delegate Custom|ListPickableItems))
  (EventDispatchers|BindEventtoToNextListedItemClicked (Variables|Default|GetOverlay) (delegate Custom|ToNextListedItem))
  (EventDispatchers|BindEventtoAddtoInventoryClicked (Variables|Default|GetOverlay) (delegate Custom|AddToInventory))
  (EventDispatchers|BindEventtoRemovefromInventoryClicked (Variables|Default|GetOverlay) (delegate Custom|RemoveFromInventory)))

(event Custom|SkipTutorialEvent
  ;[1 1 1] Key mapping section
  ;;[0 0 0] Press "T" to skip the Tutorial (without the Train if not used)
  (Transformation|SetActorLocation (Game|Player|GetPlayerPawn 0) (Variables|Default|GetFirstCampLocation) false false))

(event EventBeginPlay
  (Input|EnableInput (Game|GetPlayerController 0))
  (bind _returnvalue (UserInterface|CreateWidget "/Game/Mods/MWRandomizerMod/ModDebug/WBP_Overlay.WBP_Overlay_C"))
  (bind _output_get (Variables|Default|SetOverlay _returnvalue))
  (UserInterface|Viewport|AddtoViewport _output_get 0)
  (bind _returnvalue_2 (UserInterface|CreateWidget "/Game/Mods/MWRandomizerMod/ModDebug/WBP_ModDebugUI.WBP_ModDebugUI_C"))
  (bind _output_get_2 (Variables|Default|SetModDebugUI _returnvalue_2))
  (UserInterface|Viewport|AddtoViewport _output_get_2 0)
  (CallFunction|SetButtonEvents)
  (bind _returnvalue_3 (AddComponent|AddFloatingPawnMovement (Game|Player|GetPlayerPawn 0)))
  (Variables|Default|SetPawnMovementComponent _returnvalue_3)
  (bind _returnvalue_4 (Actor|GetActorOfClass "/Game/NaturalMovementV3/Blueprint/Character/BP_NMCharacter_Player.BP_NMCharacter_Player_C"))
  (Variables|Default|SetPlayer _returnvalue_4))

(event EventTick
  (params (DeltaSeconds :type Float%20%28single-precision%29))
  (if (Variables|Default|GetEnableVisualFeedback)
    (Variables|/Game/Mods/MWRandomizerMod/ModDebug/WBP_ModDebugUI.WBP_ModDebugUI_C|SetItemText (Variables|Default|GetModDebugUI) (Utilities|String|ToString(Vector) (.WorldLocation (CallFunction|GetWorldPlayerViewLocation))))))

(event Input|KeyboardEvents|NumPadZero
  (params (Key :type Key%20Structure :default "None"))
  ;[1 1 1] Key mapping section
  ;;[0 0 0] Press "0" to mark player's location
  (:Pressed
    (CallFunction|MarkCurrentLocation)))

(event Input|KeyboardEvents|Decimal
  (params (Key :type Key%20Structure :default "None"))
  ;[1 1 1] Testing Fogs
  (:Pressed
    (bind _returnvalue (Game|SpawnActorfromClass "/Game/Mods/MWRandomizerMod/Archipelago/CursedFog/BP_CursedFog.BP_CursedFog_C" (Math|Transform|MakeTransform "11643.290039,-21706.945312,10381.763672" "0, 0, 0" "1.700000,1.700000,1.700000") "AlwaysSpawn" 0 0))
    (Variables|Default|SetTmpTempleFog _returnvalue)))

(event Input|KeyboardEvents|Up
  (params (Key :type Key%20Structure :default "None"))
  ;[1 1 1] Testing Fogs
  (:Pressed
    (Transformation|SetActorLocation (Variables|Default|GetTmpTempleFog) (+ (Transformation|GetActorLocation (Variables|Default|GetTmpTempleFog)) "0.000000,-10.000000,0.000000") false false)))

(event Input|KeyboardEvents|T
  (params (Key :type Key%20Structure :default "None"))
  ;[1 1 1] Key mapping section
  ;;[0 0 0] Press "T" to skip the Tutorial (without the Train if not used)
  (:Pressed
    (Transformation|SetActorLocation (Game|Player|GetPlayerPawn 0) (Variables|Default|GetFirstCampLocation) false false)))

(event Input|KeyboardEvents|F
  (params (Key :type Key%20Structure :default "None"))
  (bind _pawnmovementcomponent (Variables|Default|GetPawnMovementComponent))
  ;[1 1 1] Key mapping section
  ;;[0 0 0] Press "F" to enable/disable the speed boost
  (:Pressed
    (bind _output_get (Variables|Default|SetEnableSpeedBoost (not (Variables|Default|GetEnableSpeedBoost))))
    (if _output_get
      (Variables|/Script/Engine.FloatingPawnMovement|SetMaxSpeed _pawnmovementcomponent 2e+05)
      (Variables|/Script/Engine.FloatingPawnMovement|SetAcceleration _pawnmovementcomponent 4e+03)
      (Variables|/Script/Engine.FloatingPawnMovement|SetDeceleration _pawnmovementcomponent 8e+03)
      (else
        (Variables|/Script/Engine.FloatingPawnMovement|SetMaxSpeed _pawnmovementcomponent 8e+02)
        (Variables|/Script/Engine.FloatingPawnMovement|SetAcceleration _pawnmovementcomponent 1e+06)
        (Variables|/Script/Engine.FloatingPawnMovement|SetDeceleration _pawnmovementcomponent 8e+03)))))

(event Input|KeyboardEvents|NumPadOne
  (params (Key :type Key%20Structure :default "None"))
  (bind _itemactor2 (Variables|Default|GetItemActor2))
  (bind _itemactor1 (Variables|Default|GetItemActor1))
  ;[1 1 1] Key mapping section
  ;;[0 0 0] Press "1" to swap 2 selected Actors with "R"
  (:Pressed
    ;;;[1 1 1] Check the actors to swap are valid
    (if (and (Utilities|IsValid (Variables|Default|GetItemActor1)) (Utilities|IsValid (Variables|Default|GetItemActor2)))
      (Variables|Default|SetTmpActor1Location (Transformation|GetActorLocation _itemactor1)) ; Store the location of the Actor1\nto not loose it
      (Transformation|SetActorLocation _itemactor1 (Transformation|GetActorLocation _itemactor2) false false)
      (Transformation|SetActorLocation _itemactor2 (Variables|Default|GetTmpActor1Location) false false))))

(event Input|KeyboardEvents|F1
  (params (Key :type Key%20Structure :default "None"))
  (bind _overlay (Variables|Default|GetOverlay))
  ;[1 1 1] Key mapping section
  ;;[0 0 0] Press "F1" to show the Overlay and Cursor or to hide them
  (:Pressed
    (bind _output_get (Variables|Default|SetShowOverlay (not (Variables|Default|GetShowOverlay))))
    (bind _output_get_2 (Variables|/Script/Engine.PlayerController|SetbShowMouseCursor (Game|GetPlayerController 0) _output_get))
    (if _output_get_2
      (Widget|SetVisibility _overlay "Visible")
      (else
        (Widget|SetVisibility _overlay "Hidden")))))

(event Input|KeyboardEvents|R
  (params (Key :type Key%20Structure :default "None"))
  ;[1 1 1] Key mapping section
  ;;[0 0 0] Press "R" to select an item and to get its references
  (:Pressed
    (if true
      (CallFunction|SetClickedActor))))

(event Input|KeyboardEvents|V
  (params (Key :type Key%20Structure :default "None"))
  (bind _moddebugui (Variables|Default|GetModDebugUI))
  ;[1 1 1] Key mapping section
  ;;[0 0 0] Press "V" to show the Visual Feedback
  (:Pressed
    (bind _output_get (Variables|Default|SetEnableVisualFeedback (not (Variables|Default|GetEnableVisualFeedback))))
    (if _output_get
      (Widget|SetVisibility _moddebugui "SelfHitTestInvisible")
      (else
        (Widget|SetVisibility _moddebugui "Hidden")))))

(event Input|KeyboardEvents|Add
  (params (Key :type Key%20Structure :default "None"))
  ;[1 1 1] Key mapping section
  ;;[0 0 0] Press "+" to add an item to the inventory
  (:Pressed
    (CallFunction|AllItemstoInventory 8)))

(event Input|KeyboardEvents|L
  (params (Key :type Key%20Structure :default "None"))
  ;[1 1 1] Key mapping section
  ;;[0 0 0] Press "L" to be teleported to the Lockpicks mission
  (:Pressed
    (Transformation|SetActorLocation (Game|Player|GetPlayerPawn 0) (Variables|Default|GetLockpicksMissionLocation) false false)))

(event Input|KeyboardEvents|Left
  (params (Key :type Key%20Structure :default "None"))
  ;[1 1 1] Testing Fogs
  (:Pressed
    (Transformation|SetActorLocation (Variables|Default|GetTmpTempleFog) (+ (Transformation|GetActorLocation (Variables|Default|GetTmpTempleFog)) "-10.000000, 0, 0") false false)))

(event Input|KeyboardEvents|Subtract
  (params (Key :type Key%20Structure :default "None"))
  ;[1 1 1] Key mapping section
  ;;[0 0 0] Press "-" to remove an item from the inventory
  (:Pressed
    (CallFunction|AllItemstoInventory -1)))

(event Input|KeyboardEvents|NumPadTwo
  (params (Key :type Key%20Structure :default "None"))
  ;[1 1 1] Key mapping section
  ;;[0 0 0] Press "2" to virtually list all pickable items (laggy) and to teleport on each with "3"
  (:Pressed
    (bind _outactors (Actor|GetAllActorsOfClass "/Game/_GAME/Blueprints/ItemPickup.ItemPickup_C"))
    (bind _output_get (Variables|Default|SetAllPickupItems _outactors))
    (for _array_element _output_get
      ;;[0.4243 0.7148 1] Print each found item information in the mod loader
      (CallFunction|PrinttoModLoader (Utilities|GetDisplayName _array_element))
      (CallFunction|PrinttoModLoader (Utilities|GetClassDisplayName (Utilities|GetClass _array_element)))
      (CallFunction|PrinttoModLoader (Utilities|String|ToString(Vector) (Transformation|GetActorLocation _array_element))))
    (Variables|Default|SetItemIndex 0)))

(event Input|KeyboardEvents|NumPadThree
  (params (Key :type Key%20Structure :default "None"))
  ;[1 1 1] Key mapping section
  ;;[0 0 0] Press "3" to teleport to the next listed item with "2"
  (:Pressed
    (CallFunction|TeleportPlayertoNextItem)))

(event Input|KeyboardEvents|B
  (params (Key :type Key%20Structure :default "None"))
  ;[1 1 1] Key mapping section
  ;;[0 0 0] Press "B" to be teleported back to the Train
  (:Pressed
    (Transformation|SetActorLocation (Game|Player|GetPlayerPawn 0) "0, 0, 0" false false)))

(event Input|KeyboardEvents|K
  (params (Key :type Key%20Structure :default "None"))
  ;[1 1 1] [Test module] Teleport to Bridge
  (:Pressed
    (Transformation|SetActorLocation (Game|Player|GetPlayerPawn 0) "-72000.000000,-107000.000000,11000.000000" false false)))

(event Input|KeyboardEvents|RightShift
  (params (Key :type Key%20Structure :default "None"))
  (bind _tmptemplefog (Variables|Default|GetTmpTempleFog))
  (bind _returnvalue (Transformation|GetActorTransform _tmptemplefog))
  ;[1 1 1] Testing Fogs
  (:Pressed
    (Transformation|SetActorTransform (Variables|Default|GetTmpTempleFog) (Math|Transform|MakeTransform (.location _returnvalue) "0, 0, 0" (+ (.scale _returnvalue) "0.100000,0.100000,0.100000")))))

(event Input|KeyboardEvents|Right
  (params (Key :type Key%20Structure :default "None"))
  ;[1 1 1] Testing Fogs
  (:Pressed
    (Transformation|SetActorLocation (Variables|Default|GetTmpTempleFog) (+ (Transformation|GetActorLocation (Variables|Default|GetTmpTempleFog)) "10.000000, 0, 0") false false)))

(event Input|KeyboardEvents|Asterix
  (params (Key :type Key%20Structure :default "None"))
  (bind _tmptemplefog (Variables|Default|GetTmpTempleFog))
  (bind _returnvalue (Transformation|GetActorTransform _tmptemplefog))
  ;[1 1 1] Testing Fogs
  (:Pressed
    (CallFunction|PrinttoModLoader (Utilities|String|ToString(Vector) (.location _returnvalue)))
    (CallFunction|PrinttoModLoader (Utilities|String|ToString(Vector) (.scale _returnvalue)))))

(event Input|KeyboardEvents|PageDown
  (params (Key :type Key%20Structure :default "None"))
  ;[1 1 1] Testing Fogs
  (:Pressed
    (Transformation|SetActorLocation (Variables|Default|GetTmpTempleFog) (+ (Transformation|GetActorLocation (Variables|Default|GetTmpTempleFog)) "0,0.000000,-10.000000") false false)))

(event Input|KeyboardEvents|PageUp
  (params (Key :type Key%20Structure :default "None"))
  ;[1 1 1] Testing Fogs
  (:Pressed
    (Transformation|SetActorLocation (Variables|Default|GetTmpTempleFog) (+ (Transformation|GetActorLocation (Variables|Default|GetTmpTempleFog)) "0.000000,0.000000,10.000000") false false)))

(event Input|KeyboardEvents|RightCtrl
  (params (Key :type Key%20Structure :default "None"))
  (bind _tmptemplefog (Variables|Default|GetTmpTempleFog))
  (bind _returnvalue (Transformation|GetActorTransform _tmptemplefog))
  ;[1 1 1] Testing Fogs
  (:Pressed
    (Transformation|SetActorTransform (Variables|Default|GetTmpTempleFog) (Math|Transform|MakeTransform (.location _returnvalue) "0, 0, 0" (+ (.scale _returnvalue) "-0.100000,-0.100000,-0.100000")))))

(event Input|KeyboardEvents|Down
  (params (Key :type Key%20Structure :default "None"))
  ;[1 1 1] Testing Fogs
  (:Pressed
    (Transformation|SetActorLocation (Variables|Default|GetTmpTempleFog) (+ (Transformation|GetActorLocation (Variables|Default|GetTmpTempleFog)) "0,10.000000,0.000000") false false)))

(fn ConstructionScript)

(fn TeleportPlayertoNextItem
  (while (not (Utilities|IsValid (Utilities|Array|Get(acopy) (Variables|Default|GetAllPickupItems) (Variables|Default|GetItemIndex))))
    ;[1 1 1] Increment the index until a valid item to be teleported on is found (if all array is read, return)
    (bind _result (Math|Integer|IncrementInt (Variables|Default|GetItemIndex))
      (:%20%20
        (bind _output_get (Variables|Default|SetItemIndex _result))
        (if (not (Utilities|Array|IsValidIndex (Variables|Default|GetAllPickupItems) _output_get))
          (return)))))
  (Transformation|SetActorLocation (Game|Player|GetPlayerPawn 0) (+ (Transformation|GetActorLocation (Utilities|Array|Get(acopy) (Variables|Default|GetAllPickupItems) (Variables|Default|GetItemIndex))) "0, 0,50.000000") false false)
  (bind _result_2 (Math|Integer|IncrementInt (Variables|Default|GetItemIndex))
    (:%20%20
      (Variables|Default|SetItemIndex _result_2)
      (return))))

(fn AddItemtoInventory
  (params (ItemName :type Name) (Amount :type Integer) (Show%20Notification? :type Boolean))
  (bind _returnvalue (Actor|GetActorOfClass "/Game/EasySave/easySaveObject.easySaveObject_C"))
  ;[1 1 1] Add 1 item, then add the others items following these rules :
  ; 1) If a notification must be shown, show the "add" one
  ; 2) "Gather Item" only add 1 item, "Use Item" works with more
  ; 3) Negative used items in "Use Item" add them instead of removing
  ; 4) Do not show notification "Use Item" notification (no removal)
  (Default|GatherItem _returnvalue ItemName Show%20Notification?)
  (bind _result (Math|Integer|DecrementInt Amount)
    (:%20%20
      (bind _result_2 (Utilities|NegateInt _result)
        (:%20%20
          (Default|UseItem _returnvalue ItemName _result_2 false false false)
          (CallFunction|PrinttoModLoader "Item added to inventory")
          (return))))))

(fn RemoveItemfromInventory
  (params (Name :type Name) (Amount :type Integer) (ShowNotification? :type Boolean) (PlaySound? :type Boolean))
  (bind _returnvalue (Actor|GetActorOfClass "/Game/EasySave/easySaveObject.easySaveObject_C"))
  (Default|UseItem _returnvalue Name Amount ShowNotification? false PlaySound?)
  (CallFunction|PrinttoModLoader "Item removed from inventory")
  (return))

(fn SetClickedActor
  (bind (_worldlocation _worlddirection) (CallFunction|GetWorldPlayerViewLocation))
  ;[1 1 1] Identify which actor is selected by the player (at the center of the viewport)
  (bind (_outhit _returnvalue) (Collision|LineTraceByChannel _worldlocation (+ _worldlocation (* _worlddirection (LocalVariables|GetInteractionDistance))) "TraceTypeQuery1" false (Utilities|Array|MakeArray (Game|Player|GetPlayerPawn 0)) "Persistent"))
  (if _returnvalue
    (Variables|Default|SetClickedActor (.HitActor (Collision|BreakHitResult _outhit)))
    (Variables|Default|SetClickedComponent (.HitComponent (Collision|BreakHitResult _outhit)))
    (CallFunction|UpdateAlternateActorSelection)
    (CallFunction|PrintClickedActorInformation (.Distance (Collision|BreakHitResult _outhit))) ; To enable to show all information of the clicked Actor
  ))

(fn GetWorldPlayerViewLocation
  (bind _returnvalue (Game|GetPlayerController 0))
  (bind _returnvalue_2 (Viewport|GetViewportSize))
  (bind _returnvalue_3 (/ _returnvalue_2 2.0))
  (bind (_x _y) (Math|Vector2D|BreakVector2D _returnvalue_3))
  (bind (_worldlocation _worlddirection) (Class|PlayerController|DeprojectScreenPositiontoWorld _returnvalue _x _y))
  (return _worldlocation _worlddirection))

(fn UpdateAlternateActorSelection
  (bind _clickedactor (Variables|Default|GetClickedActor))
  (bind _output_get (Variables|Default|SetSelectedActor1 (not (Variables|Default|GetSelectedActor1))))
  (if _output_get
    (Variables|Default|SetItemActor1 _clickedactor)
    (else
      (Variables|Default|SetItemActor2 _clickedactor)))
  (return))

(fn PrintClickedActorInformation
  (params (Distance :type Float%20%28single-precision%29))
  (bind _clickedactor (Variables|Default|GetClickedActor))
  (bind _clickedactor_2 (Variables|Default|GetClickedActor))
  (bind _clickedactor_3 (Variables|Default|GetClickedActor))
  (bind _clickedcomponent (Variables|Default|GetClickedComponent))
  (bind _clickedactor_4 (Variables|Default|GetClickedActor))
  (bind _clickedactor_5 (Variables|Default|GetClickedActor))
  (bind _returnvalue (Transformation|GetActorLocation _clickedactor_2))
  (bind _returnvalue_2 (Utilities|GetOuterObject _clickedactor))
  (bind _returnvalue_3 (Utilities|GetObjectName _clickedactor_5))
  (bind _returnvalue_4 (Actor|GetComponentbyClass _clickedactor_4 "/Script/Engine.PrimitiveComponent"))
  (bind _returnvalue_5 (Utilities|GetObjectName _clickedcomponent))
  (bind _returnvalue_6 (Utilities|GetClass _clickedactor_3))
  (bind _returnvalue_7 (Utilities|GetClassDisplayName _returnvalue_6))
  (bind _returnvalue_8 (Utilities|GetOuterObject _returnvalue_2))
  (bind _returnvalue_9 (Utilities|String|ToString(Vector) _returnvalue))
  (bind _returnvalue_10 (Utilities|GetObjectName _returnvalue_8))
  (LocalVariables|SetLocalDistance Distance)
  (CallFunction|PrinttoModLoader "--------") ; Separation bar
  ;[1 1 1] Print name of component
  (Development|PrintString _returnvalue_5)
  (CallFunction|PrinttoModLoader "Name of component :")
  (CallFunction|PrinttoModLoader _returnvalue_5)
  ;[1 1 1] Print name of actor
  (Development|PrintString _returnvalue_3)
  (CallFunction|PrinttoModLoader "Name of actor :")
  (CallFunction|PrinttoModLoader _returnvalue_3)
  ;[1 1 1] Print class of actor
  (Development|PrintString _returnvalue_7)
  (CallFunction|PrinttoModLoader "Class of actor :")
  (CallFunction|PrinttoModLoader _returnvalue_7)
  ;[1 1 1] Print actor location
  (Development|PrintString _returnvalue_9)
  (CallFunction|PrinttoModLoader "World location of actor :")
  (CallFunction|PrinttoModLoader _returnvalue_9)
  ;[1 1 1] Print distance to actor
  (Development|PrintString (Utilities|String|ToString(Float) (LocalVariables|GetLocalDistance)))
  (CallFunction|PrinttoModLoader "Distance to player :")
  (CallFunction|PrinttoModLoader (Utilities|String|ToString(Float) (LocalVariables|GetLocalDistance)))
  ;[1 1 1] Current level
  (Development|PrintString _returnvalue_10)
  (CallFunction|PrinttoModLoader "Level Name :")
  (CallFunction|PrinttoModLoader _returnvalue_10)
  ;[1 1 1] Show all collisions
  (CallFunction|PrinttoModLoader (Utilities|String|EnumtoString (Collision|GetCollisionEnabled _returnvalue_4)))
  (for _array_element (LocalVariables|GetCollisionChannels)
    (CallFunction|PrinttoModLoader (Utilities|String|Append (Utilities|String|EnumtoString _array_element) " : " (Utilities|String|EnumtoString (Collision|GetCollisionResponsetoChannel _returnvalue_4 _array_element)))))
  (CallFunction|PrinttoModLoader (Utilities|String|Append "Collision of this own object : " (Utilities|String|EnumtoString (Collision|GetCollisionObjectType _returnvalue_4))))
  (CallFunction|PrinttoModLoader "--------") ; Separation bar
)

(fn AllItemstoInventory
  (params (Amount :type Integer))
  (for _array_element (LocalVariables|GetTmpMissionItems)
    (CallFunction|AddItemtoInventory _array_element Amount true))
  (return))

(fn MarkCurrentLocation
  (Game|SpawnActorfromClass "/Game/_GAME/Props/Meshes/SwapableSphereActor.SwapableSphereActor_C" (Math|Transform|MakeTransform (.WorldLocation (CallFunction|GetWorldPlayerViewLocation)) "0, 0, 0" "10.000000,10.000000,10.000000") "AlwaysSpawn" 0 0)
  (CallFunction|PrinttoModLoader (Utilities|String|Append "Marked location at " (Utilities|String|ToString(Vector) (.WorldLocation (CallFunction|GetWorldPlayerViewLocation))))))